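; BP_MoveRect is a CoinGame actor that endlessly moves along a square path relative to its own orientation.
; A looping timer started at BeginPlay fires Move, which offsets the actor one unit along the right or forward vector, or their negation, selected by MoveDirection.
; After 100 units from AnchorLocation, it re-anchors and advances the direction enum with modulo wraparound.
; Two unconnected switch-based versions of the same movement remain in the graph.
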(event Custom|Move
  (Transformation|AddActorWorldOffset (Utilities|Select :Index (Variables|Default|GetMoveDirection) :NewEnumerator0 (Transformation|GetActorRightVector) :NewEnumerator1 (Transformation|GetActorForwardVector) :NewEnumerator2 (Math|Vector|NegateVector (Transformation|GetActorRightVector)) :NewEnumerator3 (Math|Vector|NegateVector (Transformation|GetActorForwardVector))))
  (if (>= (Math|Vector|VectorLength (- (Transformation|GetActorLocation) (Variables|Default|GetAnchorLocation))) 1e+02)
    (Variables|Default|SetMoveDirection (Utilities|Enum|ByteToEnumEN_MoveType (Class|KismetMathLibrary|PercentByteByte (+ (Math|Byte|MakeLiteralByte (Variables|Default|GetMoveDirection)) 1) (Math|Conversions|ToByte(Integer) (|GetNumEnumEntries)))))
    (Variables|Default|SetAnchorLocation (Transformation|GetActorLocation))))

(event EventBeginPlay
  (Variables|Default|SetAnchorLocation (Transformation|GetActorLocation))
  (Utilities|Time|SetTimerbyEvent (delegate Custom|Move) 0.005 true))

(fn ConstructionScript)